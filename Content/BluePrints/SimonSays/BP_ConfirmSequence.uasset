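; Simon Says puzzle input actor that checks hits on four coloured components against the sequence in BP_SimonSaysSequence.
; Each hit spawns a coloured Niagara burst and passes its material to CheckInput for comparison with the current step.
; A completed sequence updates the round indicator and starts a new one, until the final round opens TargetDoor.
; A wrong hit plays a sound, pulses player FOV and replaces the sequence without resetting the round.
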(event OnComponentHit(Red)
  (params (HitComponent :type Primitive%20Component%20Object%20Reference) (OtherActor :type Actor%20Object%20Reference) (OtherComp :type Primitive%20Component%20Object%20Reference) (NormalImpulse :type Vector :default "0, 0, 0") (Hit :type Hit%20Result%20Structure%20%28by%20ref%29))
  (Niagara|SpawnSystematLocation "/Game/BluePrints/SimonSays/Particles/NS_ColourHitRed.NS_ColourHitRed" (Transformation|GetWorldLocation (Variables|Default|GetRed)))
  (CallFunction|CheckInput "/Game/BluePrints/SimonSays/Materials/m_simoncolourRED.m_simoncolourRED"))

(event OnComponentHit(Blue)
  (params (HitComponent :type Primitive%20Component%20Object%20Reference) (OtherActor :type Actor%20Object%20Reference) (OtherComp :type Primitive%20Component%20Object%20Reference) (NormalImpulse :type Vector :default "0, 0, 0") (Hit :type Hit%20Result%20Structure%20%28by%20ref%29))
  (Niagara|SpawnSystematLocation "/Game/BluePrints/SimonSays/Particles/NS_ColourHitBlue.NS_ColourHitBlue" (Transformation|GetWorldLocation (Variables|Default|GetBlue)))
  (CallFunction|CheckInput "/Game/BluePrints/SimonSays/Materials/m_simoncolourBlue.m_simoncolourBlue"))

(event OnComponentHit(Green)
  (params (HitComponent :type Primitive%20Component%20Object%20Reference) (OtherActor :type Actor%20Object%20Reference) (OtherComp :type Primitive%20Component%20Object%20Reference) (NormalImpulse :type Vector :default "0, 0, 0") (Hit :type Hit%20Result%20Structure%20%28by%20ref%29))
  (Niagara|SpawnSystematLocation "/Game/BluePrints/SimonSays/Particles/NS_ColourHitGreen.NS_ColourHitGreen" (Transformation|GetWorldLocation (Variables|Default|GetGreen)))
  (CallFunction|CheckInput "/Game/BluePrints/SimonSays/Materials/m_simoncolourGreen.m_simoncolourGreen"))

(event OnComponentHit(Yellow)
  (params (HitComponent :type Primitive%20Component%20Object%20Reference) (OtherActor :type Actor%20Object%20Reference) (OtherComp :type Primitive%20Component%20Object%20Reference) (NormalImpulse :type Vector :default "0, 0, 0") (Hit :type Hit%20Result%20Structure%20%28by%20ref%29))
  (Niagara|SpawnSystematLocation "/Game/BluePrints/SimonSays/Particles/NS_ColourHitYellow.NS_ColourHitYellow" (Transformation|GetWorldLocation (Variables|Default|GetYellow)))
  (CallFunction|CheckInput "/Game/BluePrints/SimonSays/Materials/m_simoncolourYellow.m_simoncolourYellow"))

(event Custom|CheckInput
  (params (CheckValue :type Material%20Object%20Reference))
  (bind _returnvalue (Actor|GetActorOfClass "/Game/BluePrints/SimonSays/BP_SimonSaysSequence.BP_SimonSaysSequence_C"))
  (if (== (Utilities|Array|Get(acopy) (Variables|/Game/BluePrints/SimonSays/BP_SimonSaysSequence.BP_SimonSaysSequence_C|GetSequence _returnvalue) (Variables|Default|GetCheckCurrentGuess)) CheckValue)
    (Math|Integer|IncrementInt (Variables|Default|GetCheckCurrentGuess)
      (:%20%20
        (if (== (Variables|Default|GetCheckCurrentGuess) (Utilities|Array|Length (Variables|/Game/BluePrints/SimonSays/BP_SimonSaysSequence.BP_SimonSaysSequence_C|GetSequence _returnvalue)))
          (if (>= (Variables|Default|GetCurrentRound) 3)
            (Development|PrintString "Puzzle Complete")
            (Audio|PlaySoundatLocation "/Game/BluePrints/SimonSays/SoundQueues_and_Sounds/DoorOpeningMp3.DoorOpeningMp3" (Transformation|GetActorLocation) "0, 0, 0" 1.0 1.0 0.0 0 0 0 0)
            (Default|OpenDoor (Variables|Default|GetTargetDoor))
            (else
              (bind _returnvalue_2 (Actor|GetActorOfClass "/Game/BluePrints/SimonSays/BP_CurrentRoundIndicator.BP_CurrentRoundIndicator_C"))
              (Default|RoundComplete _returnvalue_2 (Variables|Default|GetCurrentRound))
              (Variables|Default|SetCheckCurrentGuess 0)
              (Math|Integer|IncrementInt (Variables|Default|GetCurrentRound)
                (:%20%20
                  (Development|PrintString "next round")
                  (Default|SequenceGenerate _returnvalue)
                  (Default|FlashColour _returnvalue)))))
          (else
            (Development|PrintString "Corect")))))
    (else
      (Audio|PlaySoundatLocation "/Game/BluePrints/SimonSays/SoundQueues_and_Sounds/SC_Incorrect.SC_Incorrect" (Transformation|GetActorLocation) "0, 0, 0" 1.0 1.0 0.0 0 0 0 0)
      (bind _asbp_first_person_character (Utilities|Casting|CastToBP_FirstPersonCharacter (Game|Player|GetPlayerPawn 0)))
      (Default|FOVpulse _asbp_first_person_character)
      (Default|SequenceGenerate _returnvalue)
      (Default|FlashColour _returnvalue)
      (Variables|Default|SetCheckCurrentGuess 0)
      (Development|PrintString "Reset"))))

(event EventBeginPlay)

(fn ConstructionScript)